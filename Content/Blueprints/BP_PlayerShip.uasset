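; BP_PlayerShip is a player-possessed flying pawn with mouse look and six-direction keyboard movement relative to its orientation.
; Key events set flags that CalculateMovementDirection combines into forward, right and up vectors, cancelling opposing keys, for Tick to feed into FloatingPawnMovement.
; As wired, D moves left and A right, and Q/E vertical movement never triggers because their presses set false.
; Space and LeftCtrl flags go unused.
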(event EventBeginPlay
  (Pawn|Possess (Game|GetPlayerController 0) self))

(event Collision|EventActorBeginOverlap
  (params (OtherActor :type Actor%20Object%20Reference)))

(event EventTick
  (params (DeltaSeconds :type Float%20%28single-precision%29))
  (Class|PawnMovementComponent|AddInputVector (Variables|Default|GetFloatingPawnMovement) (CallFunction|CalculateMovementDirection) false))

(event Input|MouseEvents|MouseX
  (params (AxisValue :type Float%20%28single-precision%29))
  ;[1 1 1] Left/Right control
  (Pawn|Input|AddControllerYawInput (* AxisValue 0.5)))

(event Input|MouseEvents|MouseY
  (params (AxisValue :type Float%20%28single-precision%29))
  ;[1 1 1] Up/Down control
  (Pawn|Input|AddControllerPitchInput (* (* AxisValue -1.0) 0.5)))

(event Input|KeyboardEvents|W
  (params (Key :type Key%20Structure :default "None"))
  (:Pressed
    (Variables|Default|SetW%20is%20Pressed true))
  (:Released
    (Variables|Default|SetW%20is%20Pressed false)))

(event Input|KeyboardEvents|S
  (params (Key :type Key%20Structure :default "None"))
  (:Pressed
    (Variables|Default|SetS%20is%20Pressed true))
  (:Released
    (Variables|Default|SetS%20is%20Pressed false)))

(event Input|KeyboardEvents|A
  (params (Key :type Key%20Structure :default "None"))
  (:Pressed
    (Variables|Default|SetA%20is%20Pressed true))
  (:Released
    (Variables|Default|SetA%20is%20Pressed false)))

(event Input|KeyboardEvents|D
  (params (Key :type Key%20Structure :default "None"))
  (:Pressed
    (Variables|Default|SetD%20is%20Pressed true))
  (:Released
    (Variables|Default|SetD%20is%20Pressed false)))

(event Input|KeyboardEvents|LeftCtrl
  (params (Key :type Key%20Structure :default "None"))
  (:Pressed
    (Variables|Default|SetLeft%20Control%20is%20Pressed true))
  (:Released
    (Variables|Default|SetLeft%20Control%20is%20Pressed false)))

(event Input|KeyboardEvents|SpaceBar
  (params (Key :type Key%20Structure :default "None"))
  (:Pressed
    (Variables|Default|SetSpace%20is%20Pressed true))
  (:Released
    (Variables|Default|SetSpace%20is%20Pressed false)))

(event Input|KeyboardEvents|Q
  (params (Key :type Key%20Structure :default "None"))
  (:Pressed
    (Variables|Default|SetQ%20is%20Pressed false))
  (:Released
    (Variables|Default|SetQ%20is%20Pressed false)))

(event Input|KeyboardEvents|E
  (params (Key :type Key%20Structure :default "None"))
  (:Pressed
    (Variables|Default|SetE%20is%20Pressed false))
  (:Released
    (Variables|Default|SetE%20is%20Pressed false)))

(fn ConstructionScript)

(fn CalculateMovementDirection
  (bind _returnvalue (Transformation|GetActorRightVector))
  (bind _returnvalue_2 (Transformation|GetActorUpVector))
  (bind _returnvalue_3 (Transformation|GetActorForwardVector))
  (Variables|Default|SetDirection_FB (select (or (and (Variables|Default|GetW%20is%20Pressed) (Variables|Default|GetS%20is%20Pressed)) (and (not (Variables|Default|GetW%20is%20Pressed)) (not (Variables|Default|GetS%20is%20Pressed)))) "0, 0, 0" (Math|Vector|SelectVector (* _returnvalue_3 -1.0) _returnvalue_3 (Variables|Default|GetS%20is%20Pressed))))
  (Variables|Default|SetDirection_LR (select (or (and (Variables|Default|GetA%20is%20Pressed) (Variables|Default|GetD%20is%20Pressed)) (and (not (Variables|Default|GetA%20is%20Pressed)) (not (Variables|Default|GetD%20is%20Pressed)))) "0, 0, 0" (Math|Vector|SelectVector (* _returnvalue -1.0) _returnvalue (Variables|Default|GetD%20is%20Pressed))))
  (Variables|Default|SetDirection_UD "0, 0, 0")
  (Variables|Default|SetDirection_UD (select (or (and (Variables|Default|GetQ%20is%20Pressed) (Variables|Default|GetE%20is%20Pressed)) (and (not (Variables|Default|GetQ%20is%20Pressed)) (not (Variables|Default|GetE%20is%20Pressed)))) "0, 0, 0" (Math|Vector|SelectVector (* _returnvalue_2 -1.0) _returnvalue_2 (Variables|Default|GetQ%20is%20Pressed))))
  (return (+ (Variables|Default|GetDirection_FB) (Variables|Default|GetDirection_LR) (Variables|Default|GetDirection_UD))))